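; BP_Ball is a physics-driven, Pong-style ball that reacts to overlaps with paddles and boundaries by rewriting its sphere's linear velocity.
; A paddle hit reverses X and sets Z to the paddle collider's Z velocity plus an incrementing BallSpeed, so BallSpeed only affects Z.
; A boundary hit replaces Z with a random value of either sign rather than reflecting it, then prints a debug string.
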(event `self.ReceiveActorBeginOverlap`
  (params (OtherActor :type "Actor Object Reference"))
  (bind _aspaddle (cast `Paddle` OtherActor)
    (:`then`
      (`self.HitPaddle` _aspaddle))
    (:`CastFailed`
      (cast `Boundary` OtherActor)
      (`self.HitBoundary`)
      (`KismetSystemLibrary.PrintString` "Hello"))))

(event `self.HitPaddle`
  (params (Paddle :type "Paddle Object Reference"))
  (bind _returnvalue (`PrimitiveComponent.GetPhysicsLinearVelocity` (`Paddle.Collider` Paddle) "None"))
  (bind _result (`/Engine/EditorBlueprintResources/StandardMacros.IncrementInt` (`self.BallSpeed`))
    (:`  `
      (bind _returnvalue_2 (`PrimitiveComponent.GetPhysicsLinearVelocity` (`self.Sphere`) "None"))
      (`PrimitiveComponent.SetPhysicsLinearVelocity` (`self.Sphere`) (`KismetMathLibrary.MakeVector` (* (.x _returnvalue_2) -1.0) (.y _returnvalue_2) (+ (.z _returnvalue) (`KismetMathLibrary.Conv_IntToDouble` _result))) false "None"))))

(event `self.HitBoundary`
  (bind _returnvalue (`PrimitiveComponent.GetPhysicsLinearVelocity` (`self.Sphere`) "None"))
  (`PrimitiveComponent.SetPhysicsLinearVelocity` (`self.Sphere`) (`KismetMathLibrary.MakeVector` (.x _returnvalue) (.y _returnvalue) (* 1.0 (`KismetMathLibrary.RandomFloatInRange` -200.0 200.0))) false "None"))

(fn `UserConstructionScript`)