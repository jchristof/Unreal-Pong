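; BP_Boundary is a Pong boundary actor that can act as a goal, chosen by an IsGoal flag.
; On BeginPlay it caches the PongGameMode.
; When an actor overlaps a goal, it prints a debug message, then destroys the actor if it is a Ball.
; IsLeftGoal then selects whether the game mode increments the AI score (left goal) or the player score.
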(event `self.ReceiveBeginPlay`
  (bind _aspong_game_mode (cast `PongGameMode` (`GameplayStatics.GetGameMode`)))
  (set `self.GameModeRef` _aspong_game_mode))

(event `self.ReceiveActorBeginOverlap`
  (params (OtherActor :type "Actor Object Reference"))
  (bind _gamemoderef (`self.GameModeRef`))
  (if (`self.IsGoal`)
    (`KismetSystemLibrary.PrintString` "Goal")
    (bind _asball (cast `Ball` OtherActor))
    (`self.K2_DestroyActor` _asball)
    (if (`self.IsLeftGoal`)
      (`PongGameMode.IncreateAIScore` _gamemoderef)
      (else
        (`PongGameMode.IncreatePlayerScore` _gamemoderef)))))

(fn `UserConstructionScript`)